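; BP_ClimbingPoint is a collectible pickup that grants a small random amount of Experience to BP_PlayerCharacter.
; Tick spins the static mesh around its yaw axis at a constant, frame-rate-independent speed.
; Overlapping the Sphere component awards the experience, plays the Achievement sound at the actor's location and destroys it.
; A randomized lifespan set on BeginPlay removes uncollected points after several minutes.
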(event OnComponentBeginOverlap(Sphere)
  (params (OverlappedComponent :type Primitive%20Component%20Object%20Reference) (OtherActor :type Actor%20Object%20Reference) (OtherComp :type Primitive%20Component%20Object%20Reference) (OtherBodyIndex :type Integer) (bFromSweep :type Boolean) (SweepResult :type Hit%20Result%20Structure%20%28by%20ref%29))
  (bind _asbp_player_character (Utilities|Casting|CastToBP_PlayerCharacter OtherActor))
  (Variables|/Game/Characters/Player/BP_PlayerCharacter.BP_PlayerCharacter_C|SetExperience _asbp_player_character (+ (Variables|/Game/Characters/Player/BP_PlayerCharacter.BP_PlayerCharacter_C|GetExperience _asbp_player_character) (Math|Random|RandomIntegerinRange 1 3)))
  (Audio|PlaySoundatLocation "/Game/Sound/Player/achievement.achievement" (Transformation|GetActorLocation) "0, 0, 0" 1.0 1.0 0.0 0 0 0)
  (Actor|DestroyActor))

(event EventBeginPlay
  (Actor|SetLifeSpan (Math|Random|RandomFloatinRange 3e+02 3.6e+02)))

(event Collision|EventActorBeginOverlap
  (params (OtherActor :type Actor%20Object%20Reference)))

(event EventTick
  (params (DeltaSeconds :type Float%20%28single-precision%29))
  (Transformation|AddRelativeRotation (Variables|Default|GetStaticMesh) (Math|Rotator|MakeRotator 0.0 0.0 (* DeltaSeconds 9e+01)) false false))

(fn ConstructionScript)