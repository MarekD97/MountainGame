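; Spline-driven environment actor that lays out a line of telephone poles with wires strung between them, built entirely in the Construction Script.
; Each spline point gets a static mesh pole, yawed 90 degrees from the spline and randomly picked from two variants with an unseeded random.
; Each segment gets three spline mesh wires, with endpoints offset from the points along forward, right and up to sit high on the poles.
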(event EventBeginPlay)

(event Collision|EventActorBeginOverlap
  (params (OtherActor :type Actor%20Object%20Reference)))

(event EventTick
  (params (DeltaSeconds :type Float%20%28single-precision%29)))

(fn ConstructionScript
  (bind _spline (Variables|Default|GetSpline))
  (bind _returnvalue (Class|SplineComponent|GetNumberOfSplineSegments _spline))
  (for _index (range 0 _returnvalue)
    (bind _transform (CallFunction|GetMeshTransform _spline _index))
    (bind _returnvalue_2 (AddComponent|AddStaticMeshComponent false _transform))
    (Components|StaticMesh|SetStaticMesh _returnvalue_2 (select (Math|Random|RandomBool) "/Game/Environment/Objects/TelephonePoles_SM_TelephonePoles_02.TelephonePoles_SM_TelephonePoles_02" "/Game/Environment/Objects/TelephonePoles_SM_TelephonePoles_01.TelephonePoles_SM_TelephonePoles_01")))
  (for _index_2 (range 0 (- _returnvalue 1))
    (CallFunction|SetWireMeshPosition _spline _index_2)))

(fn GetMeshTransform
  (params (Spline%20Component :type Spline%20Component%20Object%20Reference) (PointIndex :type Integer))
  (bind _returnvalue (Spline|GetTransformatSplinePoint Spline%20Component PointIndex "Local" false))
  (bind (_location _rotation _scale) (Math|Transform|BreakTransform _returnvalue))
  (return (Math|Transform|MakeTransform _location (Math|Rotator|MakeRotator 0.0 0.0 (+ (.Yaw (Math|Rotator|BreakRotator _rotation)) 9e+01)) _scale)))

(fn SetWireMeshPosition
  (params (SplineComponent :type Spline%20Component%20Object%20Reference) (PointIndex :type Integer))
  (bind _returnvalue (Spline|GetRotationatSplinePoint SplineComponent PointIndex "Local"))
  (bind _returnvalue_2 (+ PointIndex 1))
  (bind _returnvalue_3 (Spline|GetRotationatSplinePoint SplineComponent _returnvalue_2 "Local"))
  (for _index (range 0 2)
    (LocalVariables|SetOffset (Utilities|Select :Index _index :Option%200 3e+01 :Option%201 1.8e+02 :Option%202 -165.0))
    (bind _returnvalue_4 (AddComponent|AddSplineMeshComponent false))
    (SplineMesh|SetStartPosition _returnvalue_4 (+ (Spline|GetLocationatSplinePoint SplineComponent PointIndex "Local") (+ (* (Math|Vector|GetForwardVector _returnvalue) 2e+01) (* (Math|Vector|GetRightVector _returnvalue) (LocalVariables|GetOffset)) "0,0,865.000000")) true)
    (SplineMesh|SetEndPosition _returnvalue_4 (+ (Spline|GetLocationatSplinePoint SplineComponent _returnvalue_2 "Local") (+ (* (Math|Vector|GetRightVector _returnvalue_3) (LocalVariables|GetOffset)) (* (Math|Vector|GetForwardVector _returnvalue_3) 2e+01) "0,0,865.000000")) true)))