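; Generator actor that scatters BP_ClimbingPoint actors across the X/Z plane of a resizable, rotatable box.
; Construction sizes the box from BoxSize; at BeginPlay, its extent and Density set the grid dimensions.
; SpawnActors gives each cell a weighted random chance of a randomly jittered point, rotated with the actor and stored in PointsArray.
; A looping timer repeats spawning without clearing earlier points; DestroyActors exists but is not called here.
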(event Custom|SpawnPoints
  (CallFunction|SpawnActors (stale EventBeginPlay _x) (stale EventBeginPlay _z)))

(event EventBeginPlay
  (bind (_x _z) (CallFunction|GetNumOfChunks))
  (CallFunction|SpawnActors _x _z)
  (Utilities|Time|SetTimerbyEvent (delegate Custom|SpawnPoints) 3.6e+02 true))

(event Collision|EventActorBeginOverlap
  (params (OtherActor :type Actor%20Object%20Reference)))

(event EventTick
  (params (DeltaSeconds :type Float%20%28single-precision%29)))

(fn ConstructionScript
  (Components|Box|SetBoxExtent (Variables|Default|GetBox) (Variables|Default|GetBoxSize) true))

(fn GetNumOfChunks
  (bind _box (Variables|Default|GetBox))
  (bind _density (Variables|Default|GetDensity))
  (bind _boxextent (Variables|/Script/Engine.BoxComponent|GetBoxExtent _box))
  (bind (_x _y _z) (Math|Vector|BreakVector _boxextent))
  (return (Math|Float|Truncate (/ _x _density)) (Math|Float|Truncate (/ _z _density))))

(fn SpawnActors
  (params (X :type Integer) (Z :type Integer))
  (bind _returnvalue (Transformation|GetActorRotation))
  (bind _density (Variables|Default|GetDensity))
  (bind _box (Variables|Default|GetBox))
  (bind _density_2 (Variables|Default|GetDensity))
  (bind _returnvalue_2 (* _density 2.0))
  (bind _boxextent (Variables|/Script/Engine.BoxComponent|GetBoxExtent _box))
  (bind _returnvalue_3 (Math|Random|RandomFloatinRange 0.0 _returnvalue_2))
  (for _index (range 0 (- X 1))
    (for _index_2 (range 0 (- Z 1))
      (if (Math|Random|RandomBoolwithWeight 0.7)
        (bind _returnvalue_4 (Game|SpawnActorfromClass "/Game/Environment/Objects/BP_ClimbingPoint.BP_ClimbingPoint_C" (Math|Transform|MakeTransform (+ (- (Transformation|GetActorLocation) (Math|Vector|RotateVector (Math|Vector|MakeVector (+ (/ (.x _boxextent) 2.0) _density_2) 0.0 (+ (/ (.z _boxextent) 2.0) _density_2)) _returnvalue)) (Math|Vector|RotateVector (Math|Vector|MakeVector (- (* _index _returnvalue_2) _returnvalue_3) 0.0 (- (* _index_2 _returnvalue_2) _returnvalue_3)) _returnvalue))) "Undefined" 0 0))
        (Utilities|Array|Add (Variables|Default|GetPointsArray) _returnvalue_4)))))

(fn DestroyActors
  (bind _pointsarray (Variables|Default|GetPointsArray))
  (for _array_element _pointsarray
    (Actor|DestroyActor _array_element)
    (if (Game|IsActorBeingDestroyed _array_element)
      (Utilities|Array|RemoveItem _pointsarray _array_element))))