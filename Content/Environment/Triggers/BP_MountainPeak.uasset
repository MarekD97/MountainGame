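; Mountain summit trigger that plays a celebration cinematic when the player character overlaps it.
; On overlap it hides its billboard, disables input, triggers the Cheer animation and blends the view to itself, then swings its spring arm half a turn.
; The view then returns to the player, a WBP_Quest widget reports the Experience earned climbing, and the player teleports to a target point with input restored.
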(event EventBeginPlay)

(event Collision|EventActorBeginOverlap
  (params (OtherActor :type Actor%20Object%20Reference))
  (bind _returnvalue (Game|GetPlayerController 0))
  (bind _targetpoint (Variables|Default|GetTargetPoint))
  (bind _asbp_player_character (Utilities|Casting|CastToBP_PlayerCharacter OtherActor))
  (Development|SetHiddeninGame (Variables|Default|GetBillboard) true true)
  (Input|DisableInput _asbp_player_character (.AsPlayer%20Controller (Utilities|Casting|CastToPlayerController (Pawn|GetController _asbp_player_character))))
  (bind _asplayer_anim_instance (Utilities|Casting|CastToPlayerAnimInstance (Components|SkeletalMesh|GetAnimInstance (Variables|/Script/Engine.Character|GetMesh _asbp_player_character))))
  (Class|PlayerAnimInstance|Cheer _asplayer_anim_instance)
  (Game|Player|SetViewTargetwithBlend _returnvalue self 3.0 "VTBlend_EaseIn" 1.0 true)
  (Utilities|FlowControl|Delay 3.0)
  (Components|MoveComponentTo (Variables|Default|GetSpringArm) "0, 0, 0" "-20.000000,180.000000,0.000000" true true 5.0 false)
  (Game|Player|SetViewTargetwithBlend _returnvalue _asbp_player_character 1.0 "VTBlend_EaseOut" 1.0 true)
  (Transformation|SetRelativeRotation (Variables|Default|GetSpringArm) "-20.000000, 0, 0" false false)
  (bind _returnvalue_2 (UserInterface|CreateWidget "/Game/UI/WBP_Quest.WBP_Quest_C" 0 (Variables|Default|GetImage) (Utilities|Text|FormatText "Podczas wspinaczki zdobyto {Number} punktów." (Variables|/Game/Characters/Player/BP_PlayerCharacter.BP_PlayerCharacter_C|GetExperience _asbp_player_character)) (Variables|Default|GetTitle)))
  (UserInterface|Viewport|AddtoViewport _returnvalue_2 0)
  (Transformation|SetActorLocationAndRotation _asbp_player_character (Transformation|GetActorLocation _targetpoint) (Transformation|GetActorRotation _targetpoint))
  (Input|EnableInput _asbp_player_character (.AsPlayer%20Controller (Utilities|Casting|CastToPlayerController (Pawn|GetController _asbp_player_character)))))

(event EventTick
  (params (DeltaSeconds :type Float%20%28single-precision%29)))

(fn ConstructionScript)