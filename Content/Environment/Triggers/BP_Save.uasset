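; BP_Save is a trigger actor that autosaves the game through BP_GameInstance when it is overlapped.
; A gate opens two seconds after BeginPlay and never closes, so every later overlap by any actor fires the sequence.
; The sequence shows WBP_SaveMenu, briefly blends the view to this actor, saves to "AutoSave" with an achievement sound, then blends back to the player character.
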(event EventBeginPlay
  (Utilities|FlowControl|Delay 2.0)
  (Utilities|FlowControl|Gate true) ; enters at Open
)

(event Collision|EventActorBeginOverlap
  (params (OtherActor :type Actor%20Object%20Reference))
  (Utilities|FlowControl|Gate true
    (:Exit
      (bind _returnvalue (UserInterface|CreateWidget "/Game/UI/WBP_SaveMenu.WBP_SaveMenu_C" (Game|GetPlayerController 0)))
      (UserInterface|Viewport|AddtoViewport _returnvalue 0)
      (bind _asbp_game_instance (Utilities|Casting|CastToBP_GameInstance (Game|GetGameInstance)))
      (Game|Player|SetViewTargetwithBlend (Game|GetPlayerController 0) self 0.5 "VTBlend_Linear" 0.0 false)
      (Utilities|FlowControl|Delay 0.3)
      (Default|SaveGame _asbp_game_instance "AutoSave")
      (Audio|SpawnSound2D "/Game/Sound/Player/achievement.achievement" 1.0 1.0 0.0 0)
      (Utilities|FlowControl|Delay 0.7)
      (Game|Player|SetViewTargetwithBlend (Game|GetPlayerController 0) (Game|GetPlayerCharacter 0) 0.5 "VTBlend_Linear" 0.0 false))))

(event EventTick
  (params (DeltaSeconds :type Float%20%28single-precision%29)))

(fn ConstructionScript)