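; BP_PlayerHUD is the player's HUD, which creates and manages the gameplay and quest message widgets.
; On BeginPlay it activates gameplay, creating WBP_Gameplay if none is valid; deactivating removes and clears it.
; ToggleWeatherDebug uses a FlipFlop to show or collapse that widget's weather display.
; ShowMessage spawns a new WBP_Quest popup with a title, content and image.
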(event Custom|ToggleWeatherDebug
  (bind _aswbp_gameplay (Utilities|Casting|CastToWBP_Gameplay (Variables|Default|GetGameplayWidget)))
  (Utilities|FlowControl|FlipFlop
    (:A
      (Default|SetWeatherVisibility _aswbp_gameplay "Visible"))
    (:B
      (Default|SetWeatherVisibility _aswbp_gameplay "Collapsed"))))

(event Custom|ShowMessage
  (params (Title :type Text) (Content :type Text) (Image :type Texture%202D%20Object%20Reference))
  (bind _returnvalue (UserInterface|CreateWidget "/Game/UI/WBP_Quest.WBP_Quest_C" (Variables|Default|GetPlayerOwner) Image Content Title))
  (UserInterface|Viewport|AddtoViewport _returnvalue 0))

(event Custom|SetGameplayActive
  (params (NewActive :type Boolean))
  (if NewActive
    (Variables|Default|GetGameplayWidget
      (:then)
      (:else
        (bind _returnvalue (UserInterface|CreateWidget "/Game/UI/WBP_Gameplay.WBP_Gameplay_C" (Variables|Default|GetPlayerOwner)))
        (bind _output_get (Variables|Default|SetGameplayWidget _returnvalue))
        (UserInterface|Viewport|AddtoViewport _output_get 0)))
    (else
      (bind _gameplaywidget (Variables|Default|GetGameplayWidget)
        (:then
          (Widget|RemovefromParent _gameplaywidget)
          (Variables|Default|SetGameplayWidget 0))
        (:else)))))

(event EventBeginPlay
  (CallFunction|SetGameplayActive true))

(event Collision|EventActorBeginOverlap
  (params (OtherActor :type Actor%20Object%20Reference)))

(event EventTick
  (params (DeltaSeconds :type Float%20%28single-precision%29)))

(fn ConstructionScript)