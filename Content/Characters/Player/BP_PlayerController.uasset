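; Player controller that manages pause, inventory and game-over screens, plus a weather debug toggle through the HUD.
; A shared SetUIMode switches character input, cursor and input mode, while pause and death also deactivate gameplay on BP_PlayerHUD.
; Inventory is blocked while in a shop and also spawns or destroys a BP_Wardrobe actor at the player's transform to show the character image.
; Resuming by key delegates to the pause widget's ResumeGame.
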(event Custom|ShowCharacterImage
  (bind _returnvalue (Game|GetPlayerCharacter 0))
  (bind _wardroberef (Variables|Default|GetWardrobeRef)
    (:then
      (Actor|DestroyActor _wardroberef))
    (:else
      (bind _returnvalue_2 (Game|SpawnActorfromClass "/Game/Develop/BP_Wardrobe.BP_Wardrobe_C" (Transformation|GetActorTransform _returnvalue) "Undefined" 0 _returnvalue 0))
      (Variables|Default|SetWardrobeRef _returnvalue_2))))

(event Custom|SetUIMode
  (params (Enabled :type Boolean) (WidgetToFocus :type Widget%20Object%20Reference))
  (bind _self self)
  (if Enabled
    (Input|DisableInput (Variables|Default|GetCharacterRef) _self)
    (Variables|Default|SetbShowMouseCursor true)
    (Input|SetInputModeGameandUI _self WidgetToFocus "DoNotLock" true)
    (else
      (Input|EnableInput (Variables|Default|GetCharacterRef) self)
      (Variables|Default|SetbShowMouseCursor false)
      (Input|SetInputModeGameOnly self))))

(event Custom|TogglePauseGame
  (bind _returnvalue (HUD|GetHUD))
  (bind _asbp_player_hud (Utilities|Casting|CastToBP_PlayerHUD _returnvalue))
  (Variables|Default|GetPauseMenuWidget
    (:then
      (Variables|Default|SetPauseMenuWidget 0)
      (CallFunction|SetUIMode false)
      (Game|SetGamePaused false)
      (Default|SetGameplayActive _asbp_player_hud true))
    (:else
      (bind _returnvalue_2 (UserInterface|CreateWidget "/Game/UI/WBP_PauseMenu.WBP_PauseMenu_C" self))
      (bind _output_get (Variables|Default|SetPauseMenuWidget _returnvalue_2))
      (UserInterface|Viewport|AddtoViewport _output_get 0)
      (CallFunction|SetUIMode true _output_get)
      (Game|SetGamePaused true)
      (Default|SetGameplayActive _asbp_player_hud false))))

(event Custom|ToggleInventory
  (if (not (Variables|Default|GetIsInShop))
    (CallFunction|ShowCharacterImage)
    (bind _inventorywidget (Variables|Default|GetInventoryWidget)
      (:then
        (Widget|RemovefromParent _inventorywidget)
        (Variables|Default|SetInventoryWidget 0)
        (CallFunction|SetUIMode false))
      (:else
        (bind _returnvalue (UserInterface|CreateWidget "/Game/UI/Inventory/WBP_Inventory.WBP_Inventory_C" self))
        (bind _output_get (Variables|Default|SetInventoryWidget _returnvalue))
        (UserInterface|Viewport|AddtoViewport _output_get 0)
        (CallFunction|SetUIMode true _output_get)))))

(event EventBeginPlay
  (bind _asplayer_character (Utilities|Casting|CastToPlayerCharacter (Pawn|GetControlledPawn)))
  (Variables|Default|SetCharacterRef _asplayer_character))

(event EventTick
  (params (DeltaSeconds :type Float%20%28single-precision%29)))

(event EventDie
  (Default|SetGameplayActive (.AsBP%20Player%20HUD (Utilities|Casting|CastToBP_PlayerHUD (HUD|GetHUD))) false)
  (bind _returnvalue (UserInterface|CreateWidget "/Game/UI/WBP_GameOver.WBP_GameOver_C" self))
  (UserInterface|Viewport|AddtoViewport _returnvalue 0)
  (CallFunction|SetUIMode true _returnvalue))

(event Input|ActionEvents|InputActionPauseGame
  (params (Key :type Key%20Structure :default "None"))
  (:Pressed
    (if (not (Game|IsGamePaused))
      (CallFunction|TogglePauseGame)
      (else
        (bind _pausemenuwidget (Variables|Default|GetPauseMenuWidget)
          (:then
            (if (UserInterface|Viewport|IsinViewport _pausemenuwidget)
              (bind _aswbp_pause_menu (Utilities|Casting|CastToWBP_PauseMenu _pausemenuwidget))
              (Default|ResumeGame _aswbp_pause_menu)))
          (:else))))))

(event Input|ActionEvents|InputActionInventory
  (params (Key :type Key%20Structure :default "None"))
  (:Pressed
    (if (not (Variables|Default|GetIsInShop))
      (CallFunction|ShowCharacterImage)
      (bind _inventorywidget (Variables|Default|GetInventoryWidget)
        (:then
          (Widget|RemovefromParent _inventorywidget)
          (Variables|Default|SetInventoryWidget 0)
          (CallFunction|SetUIMode false))
        (:else
          (bind _returnvalue (UserInterface|CreateWidget "/Game/UI/Inventory/WBP_Inventory.WBP_Inventory_C" self))
          (bind _output_get (Variables|Default|SetInventoryWidget _returnvalue))
          (UserInterface|Viewport|AddtoViewport _output_get 0)
          (CallFunction|SetUIMode true _output_get))))))

(event Input|KeyboardEvents|Slash
  (params (Key :type Key%20Structure :default "None"))
  (:Pressed
    (bind _asbp_player_hud (Utilities|Casting|CastToBP_PlayerHUD (HUD|GetHUD)))
    (Default|ToggleWeatherDebug _asbp_player_hud)
    (CallFunction|SetUIMode (not (Variables|Default|GetbShowMouseCursor)) (Variables|/Game/Core/BP_PlayerHUD.BP_PlayerHUD_C|GetGameplayWidget _asbp_player_hud))))

(fn ConstructionScript)