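; Player character Blueprint for climbing, linking inventory items to the climbing component and reacting to time and season.
; While climbing, left hand spends magnesia for extra climbing time and right hand hooks the rope, using an inventory hook if none exists.
; BP_SkyActor drives winter clothing at BeginPlay and per-tick soundtrack day/night and smoothed season parameters.
; Debug keys save the game and toggle climbing traces.
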(event EventTick
  (params (DeltaSeconds :type Float%20%28single-precision%29))
  (|CallParentFunction DeltaSeconds)
  (CallFunction|UpdateMusic (Variables|Default|GetSkyActor)))

(event EventBeginPlay
  (|CallParentFunction)
  (bind _returnvalue (Actor|GetActorOfClass "/Game/Environment/Climate/BP_SkyActor.BP_SkyActor_C"))
  (bind _output_get (Variables|Default|SetSkyActor _returnvalue))
  (if (> (Variables|/Script/MountainExpedition.WeatherComponent|GetCurrentSeason (Variables|/Game/Environment/Climate/BP_SkyActor.BP_SkyActor_C|GetWeather _output_get)) 1)
    (CallFunction|EquipWinterCloths)))

(event Input|ActionEvents|InputActionUseLeftHand
  (params (Key :type Key%20Structure :default "None"))
  (:Pressed
    (CallFunction|UseMagnesia)))

(event Input|ActionEvents|InputActionUseRightHand
  (params (Key :type Key%20Structure :default "None"))
  (:Pressed
    (CallFunction|PlaceHook)))

(event Input|KeyboardEvents|0
  (params (Key :type Key%20Structure :default "None"))
  (bind _climbingcomponent (Variables|Default|GetClimbingComponent))
  (:Pressed
    (Utilities|FlowControl|FlipFlop
      (:A
        (Variables|/Script/MountainExpedition.ClimbingComponent|SetDrawDebugTraceType _climbingcomponent "ForOneFrame"))
      (:B
        (Variables|/Script/MountainExpedition.ClimbingComponent|SetDrawDebugTraceType _climbingcomponent "None")))))

(event Input|KeyboardEvents|LeftCtrl
  (params (Key :type Key%20Structure :default "None"))
  ;[1 1 1] Debug
)

(event Input|KeyboardEvents|LeftAlt
  (params (Key :type Key%20Structure :default "None"))
  ;[1 1 1] SlowMo
)

(event Input|KeyboardEvents|1
  (params (Key :type Key%20Structure :default "None"))
  ;[1 1 1] Debug
  ;;[1 1 1] Save Game
  (:Pressed
    (bind _asbp_game_instance (Utilities|Casting|CastToBP_GameInstance (Game|GetGameInstance)))
    (Default|SaveGame _asbp_game_instance "Save")))

(event Input|KeyboardEvents|2
  (params (Key :type Key%20Structure :default "None"))
  ;[1 1 1] Debug
  ;;[1 1 1] Delete Game
)

(fn ConstructionScript)

(fn PlaceHook
  (bind _climbingcomponent (Variables|Default|GetClimbingComponent))
  (if (Variables|/Script/MountainExpedition.ClimbingComponent|GetbIsClimbing _climbingcomponent)
    (Variables|/Script/MountainExpedition.ClimbingComponent|GetRopeActor _climbingcomponent
      (:then
        (Class|ClimbingComponent|HookRope (Variables|Default|GetClimbingComponent)))
      (:else
        (bind _array_element (Utilities|Array|ForEachLoopwithBreak (Variables|/Script/MountainExpedition.InventoryComponent|GetItems (Variables|Default|GetInventoryComponent)) :!label _label)
          (:LoopBody
            (if (== (Utilities|GetClass _array_element) "/Game/Items/BP_Hook.BP_Hook_C")
              (Class|PlayerCharacter|UseItem _array_element)
              (Class|ClimbingComponent|HookRope (Variables|Default|GetClimbingComponent))
              (goto _label Break))))))))

(fn UpdateMusic
  (params (SkyActor :type BP%20Sky%20Actor%20Object%20Reference))
  (bind _weather (Variables|/Game/Environment/Climate/BP_SkyActor.BP_SkyActor_C|GetWeather SkyActor))
  (bind _daynight (Variables|/Game/Environment/Climate/BP_SkyActor.BP_SkyActor_C|GetDayNight SkyActor))
  (bind (_hours _minutes) (Class|DayNightComponent|GetWorldTime _daynight))
  (bind _currentseason (Variables|/Script/MountainExpedition.WeatherComponent|GetCurrentSeason _weather))
  (bind _soundtrackaudio (Variables|Default|GetSoundtrackAudio)
    (:then
      (Audio|Parameter|SetFloatParameter _soundtrackaudio "DayNight" (+ (Math|Conversions|ToFloat(Integer) _hours) (/ (Math|Conversions|ToFloat(Integer) _minutes) 6e+01)) :!class /Script/Engine.AudioComponent)
      (bind _output_get (Variables|Default|SetCurrentSeasonMusic (Math|Float|Lerp (Variables|Default|GetCurrentSeasonMusic) (Math|Float|SelectFloat 0.0 1.0 (or (Utilities|Enum|Equal(Enum) _currentseason "Spring") (Utilities|Enum|Equal(Enum) _currentseason "Summer"))) (Utilities|Time|GetWorldDeltaSeconds))))
      (Audio|Parameter|SetFloatParameter _soundtrackaudio "Season" _output_get :!class /Script/Engine.AudioComponent))
    (:else)))

(fn UseMagnesia
  (if (Variables|/Script/MountainExpedition.ClimbingComponent|GetbIsClimbing (Variables|Default|GetClimbingComponent))
    (bind _array_element (Utilities|Array|ForEachLoopwithBreak (Variables|/Script/MountainExpedition.InventoryComponent|GetItems (Variables|Default|GetInventoryComponent)) :!label _label)
      (:LoopBody
        (if (== (Utilities|GetClass _array_element) "/Game/Items/BP_Magnesia.BP_Magnesia_C")
          (Class|InventoryComponent|RemoveItem (Variables|Default|GetInventoryComponent) _array_element)
          (Class|ClimbingComponent|AddClimbingTime (Variables|Default|GetClimbingComponent) 1.0)
          (goto _label Break))))))

(fn EquipWinterCloths
  (bind _returnvalue (Game|ConstructObjectfromClass "/Game/Items/BP_Jacket.BP_Jacket_C" self))
  (Class|PlayerCharacter|UseItem _returnvalue)
  (bind _returnvalue_2 (Game|ConstructObjectfromClass "/Game/Items/BP_WinterHat.BP_WinterHat_C" self))
  (Class|PlayerCharacter|UseItem _returnvalue_2))