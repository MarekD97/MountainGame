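; BP_Pathway is a spline waypoint path, filed under Coach, that picks the next point to move to toward a target.
; The construction script puts a billboard on each spline point as a marker.
; GetNextLocation finds the point closest to the current location, then picks whichever neighbor is nearer the target in 2D, checking forward first.
; When the previous point exists but neither neighbor improves, it returns index+1, even past the last point.
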(event EventBeginPlay)

(event Collision|EventActorBeginOverlap
  (params (OtherActor :type Actor%20Object%20Reference)))

(event EventTick
  (params (DeltaSeconds :type Float%20%28single-precision%29)))

(fn ConstructionScript
  (for _index (range 0 (- (Spline|GetNumberOfSplinePoints (Variables|Default|GetSpline)) 1))
    (AddComponent|AddBillboardComponent false (Math|Transform|MakeTransform (Spline|GetLocationatSplinePoint (Variables|Default|GetSpline) _index "Local")))))

(fn GetNextLocation
  (params (TargetLocation :type Vector) (CurrentLocation :type Vector))
  (bind _spline (Variables|Default|GetSpline))
  (bind _pointindex (CallFunction|GetClosestPointIndex CurrentLocation))
  (if (< (+ _pointindex 1) (Spline|GetNumberOfSplinePoints (Variables|Default|GetSpline)))
    (if (< (Math|Vector|Distance2D(Vector) TargetLocation (Spline|GetLocationatSplinePoint _spline (+ _pointindex 1) "World")) (Math|Vector|Distance2D(Vector) TargetLocation (Spline|GetLocationatSplinePoint _spline _pointindex "World")))
      (return (Spline|GetLocationatSplinePoint _spline (+ _pointindex 1) "World"))
      (else
        _)))
  (if (>= (- _pointindex 1) 0)
    (if (< (Math|Vector|Distance2D(Vector) TargetLocation (Spline|GetLocationatSplinePoint _spline (- _pointindex 1) "World")) (Math|Vector|Distance2D(Vector) TargetLocation (Spline|GetLocationatSplinePoint _spline _pointindex "World")))
      (return (Spline|GetLocationatSplinePoint _spline (- _pointindex 1) "World"))
      (else
        (return (Spline|GetLocationatSplinePoint _spline (+ _pointindex 1) "World"))))))

(fn GetClosestPointIndex
  (params (CurrentLocation :type Vector))
  (for _index (range 0 (- (Spline|GetNumberOfSplinePoints (Variables|Default|GetSpline)) 1))
    (if (== _index 0)
      (LocalVariables|SetDistance (Math|Vector|Distance2D(Vector) (Spline|GetLocationatSplinePoint (Variables|Default|GetSpline) _index "World") CurrentLocation))
      (LocalVariables|SetIndex _index)
      (elif (< (Math|Vector|Distance2D(Vector) (Spline|GetLocationatSplinePoint (Variables|Default|GetSpline) _index "World") CurrentLocation) (LocalVariables|GetDistance))
        (LocalVariables|SetDistance (Math|Vector|Distance2D(Vector) (Spline|GetLocationatSplinePoint (Variables|Default|GetSpline) _index "World") CurrentLocation))
        (LocalVariables|SetIndex _index))))
  (return (LocalVariables|GetIndex)))

(fn PrintSomething
  (Development|PrintString "Hello"))