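; Coach character Blueprint built from modular backpack, torso and headwear meshes that follow the main mesh through master pose.
; On BeginPlay it reads the season from BP_SkyActor's weather and swaps to a jacket and red hat in later seasons.
; Tick mirrors the Quest's Enabled flag into IsReadyToGo.
; CharacterSphereTracer sphere-traces around the coach for other pawns and returns the first hit's location.
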(event EventBeginPlay
  (bind _returnvalue (Actor|GetActorOfClass "/Game/Environment/Climate/BP_SkyActor.BP_SkyActor_C"))
  (if (> (Variables|/Script/MountainExpedition.WeatherComponent|GetCurrentSeason (Variables|/Game/Environment/Climate/BP_SkyActor.BP_SkyActor_C|GetWeather _returnvalue)) 1)
    (Class|SkinnedMeshComponent|SetSkeletalMesh (Variables|Default|GetTorso) "/Game/Characters/Player/BodyParts/Jacket.Jacket" true)
    (Class|SkinnedMeshComponent|SetSkeletalMesh (Variables|Default|GetHeadwear) "/Game/Characters/Player/BodyParts/RedHat.RedHat" true)))

(event Collision|EventActorBeginOverlap
  (params (OtherActor :type Actor%20Object%20Reference)))

(event EventTick
  (params (DeltaSeconds :type Float%20%28single-precision%29))
  (bind _quest (Variables|Default|GetQuest)
    (:then
      (Variables|Default|SetIsReadyToGo (Variables|/Script/MountainExpedition.PlayerQuest|GetbEnabled _quest)))
    (:else)))

(fn ConstructionScript
  (Class|SkinnedMeshComponent|SetMasterPoseComponent (Variables|Default|GetBackpack) (Variables|Character|GetMesh) false))

(fn CharacterSphereTracer
  (bind _returnvalue (Transformation|GetActorLocation))
  (bind (_outhits _returnvalue_2) (Collision|MultiSphereTraceForObjects _returnvalue _returnvalue 1024.0 (Utilities|Array|MakeArray "ObjectTypeQuery3") false (Utilities|Array|MakeArray self) "None"))
  (if _returnvalue_2
    (for _array_element _outhits
      (return true (Transformation|GetActorLocation (.HitActor (Collision|BreakHitResult _array_element)))))
    (else
      (return false "0, 0, 0"))))