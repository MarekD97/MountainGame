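; BP_Shop is a shop actor that opens the WBP_Hostel interface when the player character walks into its Box trigger.
; On overlap it hides the character, flags the controller as in-shop, enables UI mode and blends the camera to itself.
; ExitFromShop reverses this, also unpausing the game and turning the character 180 degrees in yaw before blending the view back.
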(event OnComponentBeginOverlap(Box)
  (params (OverlappedComponent :type Primitive%20Component%20Object%20Reference) (OtherActor :type Actor%20Object%20Reference) (OtherComp :type Primitive%20Component%20Object%20Reference) (OtherBodyIndex :type Integer) (bFromSweep :type Boolean) (SweepResult :type Hit%20Result%20Structure%20%28by%20ref%29))
  (bind _asplayer_character (Utilities|Casting|CastToPlayerCharacter OtherActor))
  (bind _output_get (Variables|Default|SetPlayerRef _asplayer_character))
  (Utilities|FlowControl|Sequence
    (:then_0
      (bind _asbp_player_controller (Utilities|Casting|CastToBP_PlayerController (Pawn|GetController _output_get)))
      (bind _returnvalue (UserInterface|CreateWidget "/Game/UI/Inventory/WBP_Hostel.WBP_Hostel_C" _asbp_player_controller self))
      (UserInterface|Viewport|AddtoViewport _returnvalue 0)
      (Variables|/Game/Characters/Player/BP_PlayerController.BP_PlayerController_C|SetIsInShop _asbp_player_controller true))
    (:then_1
      (Rendering|SetActorHiddenInGame _output_get true)
      (bind _asbp_player_controller_2 (Utilities|Casting|CastToBP_PlayerController (Game|GetPlayerController 0)))
      (Default|SetUIMode _asbp_player_controller_2 true _returnvalue)
      (Game|Player|SetViewTargetwithBlend (Game|GetPlayerController 0) self 1.0 "VTBlend_Linear" 0.0 false))))

(event Custom|ExitFromShop
  (bind _playerref (Variables|Default|GetPlayerRef))
  (bind _returnvalue (Transformation|GetActorRotation _playerref))
  (bind (_roll _pitch _yaw) (Math|Rotator|BreakRotator _returnvalue))
  (bind _playerref_2 (Variables|Default|GetPlayerRef)
    (:then
      (Rendering|SetActorHiddenInGame _playerref_2 false)
      (Game|SetGamePaused false)
      (bind _asbp_player_controller (Utilities|Casting|CastToBP_PlayerController (Game|GetPlayerController 0)))
      (Variables|/Game/Characters/Player/BP_PlayerController.BP_PlayerController_C|SetIsInShop _asbp_player_controller false)
      (Default|SetUIMode _asbp_player_controller false)
      (Transformation|SetActorRotation _playerref (Math|Rotator|MakeRotator _roll _pitch (+ _yaw 1.8e+02)))
      (Game|Player|SetViewTargetwithBlend (Game|GetPlayerController 0) (Game|GetPlayerCharacter 0) 1.0 "VTBlend_Linear" 0.0 false))
    (:else)))

(event EventBeginPlay)

(event EventTick
  (params (DeltaSeconds :type Float%20%28single-precision%29)))

(fn ConstructionScript)